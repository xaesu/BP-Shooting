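; BP_Bullet is a projectile actor that flies straight ahead and destroys enemies it hits.
; Tick moves it along its forward vector by MoveSpeed scaled by delta time, without sweep, so hits rely on overlap events.
; On overlapping a BP_Enemy it destroys the enemy, spawns an explosion emitter at its own location, adds one point through BP_GameModeBase, then destroys itself.
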(event EventBeginPlay)

(event Collision|EventActorBeginOverlap
  (params (OtherActor :type Actor%20Object%20Reference))
  (bind _asbp_enemy (Utilities|Casting|CastToBP_Enemy OtherActor))
  (Actor|DestroyActor _asbp_enemy)
  ;[1 1 1] 파티클 생성 로드 - 생성 위치 충돌한 위치에서 액터 자신의 위치로 설정
  (Effects|SpawnEmitteratLocation "/Game/StarterContent/Particles/P_Explosion.P_Explosion" (Transformation|GetActorLocation))
  ;[1 1 1] 총알이 적을 맞출 때마다 1점씩 점수 누적
  (bind _asbp_game_mode_base (Utilities|Casting|CastToBP_GameModeBase (Game|GetGameMode)))
  (Default|AddScore _asbp_game_mode_base 1)
  (Actor|DestroyActor))

(event EventTick
  (params (DeltaSeconds :type Float%20%28single-precision%29))
  ;[1 1 1] 총알 전방 이동 처리
  ; 상대좌표 기준으로 처리해야하므로 벡터 기준(MakeVector) 노드 제외
  (Transformation|SetActorLocation (+ (Transformation|GetActorLocation) (* (* (Transformation|GetActorForwardVector) (Variables|Default|GetMoveSpeed)) DeltaSeconds)) false false))

(fn ConstructionScript)