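; BP_Enemy is an enemy that flies in a straight line and destroys the player on contact.
; At BeginPlay a TraceRate roll chooses between its forward vector and a player-based direction, computed from player location minus its forward vector rather than its own location.
; Tick moves it along that fixed direction at MoveSpeed without sweeping.
; Overlapping BP_Player destroys the player, spawns a steam particle at the enemy and destroys itself.
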(event EventBeginPlay
  (if (<= (Math|Random|RandomFloatinRange 0.0 1.0) (Variables|Default|GetTraceRate))
    ;[1 1 1] 조건문의 조건이 True 일 때, 실행
    ;;[1 1 1] 월드 공간에서 이동 중인 위치 파악
    (bind _returnvalue (Actor|GetActorOfClass "/Game/Blueprints/BP_Player.BP_Player_C"))
    (Utilities|IsValid _returnvalue
      (:Is%20Valid
        (Variables|Default|SetDirection (Math|Vector|Normalize (- (Transformation|GetActorLocation _returnvalue) (Transformation|GetActorForwardVector))))))
    (else
      ;[1 1 1] 조건문의 조건이 False 일 때, 실행
      (Variables|Default|SetDirection (Transformation|GetActorForwardVector)))))

(event Collision|EventActorBeginOverlap
  (params (OtherActor :type Actor%20Object%20Reference))
  (bind _asbp_player (Utilities|Casting|CastToBP_Player OtherActor))
  (Actor|DestroyActor _asbp_player)
  ;[1 1 1] 파티클 생성 로드 - 생성 위치 충돌한 위치에서 액터 자신의 위치로 설정
  (Effects|SpawnEmitteratLocation "/Game/StarterContent/Particles/P_Steam_Lit.P_Steam_Lit" (Transformation|GetActorLocation))
  (Actor|DestroyActor))

(event EventTick
  (params (DeltaSeconds :type Float%20%28single-precision%29))
  (Transformation|SetActorLocation (+ (Transformation|GetActorLocation) (* (* (Variables|Default|GetDirection) (Variables|Default|GetMoveSpeed)) DeltaSeconds)) false false))

(fn ConstructionScript)