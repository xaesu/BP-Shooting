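; Game mode that shows the main HUD widget and tracks the current score and a persistent best score.
; On BeginPlay it adds BP_MainWidget to the viewport and loads BestScore from the BestScoreData save slot.
; AddScore accumulates points and saves any new best through a fresh BP_SaveScore object.
; LoadScoreData's existence check uses an empty slot name and its result is unused, so loading is always attempted.
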(event EventBeginPlay
  ;[1 1 1] 위젯을 메모리 공간에 로드
  (bind _returnvalue (UserInterface|CreateWidget "/Game/UI/BP_MainWidget.BP_MainWidget_C"))
  (UserInterface|Viewport|AddtoViewport _returnvalue 0)
  (bind _best_score (CallFunction|LoadScoreData))
  (Variables|Default|SetBestScore _best_score))

(event EventTick
  (params (DeltaSeconds :type Float%20%28single-precision%29)))

(fn ConstructionScript)

(fn AddScore
  (params (Point :type Integer))
  ;[1 1 1] 점수 누적
  ;[1 1 1] 현재 점수가 기존 최고 점수보다 클 때,
  (bind _output_get (Variables|Default|SetCurrentScore (+ Point (Variables|Default|GetCurrentScore))))
  (if (> _output_get (Variables|Default|GetBestScore))
    (bind _output_get_2 (Variables|Default|SetBestScore _output_get))
    ;[1 1 1] 점수 데이터 저장
    (CallFunction|SaveScoreData _output_get_2)))

(fn SaveScoreData
  (params (SaveValue :type Integer))
  ;[1 1 1] 컴퓨기 메모리에 인스턴스 형태로 임시로 존재하는 세이브 데이터를 변수 형태로 다루기 위해 구체적인 변수 형태로 승격
  (bind _returnvalue (SaveGame|CreateSaveGameObject "/Game/Blueprints/BP_SaveScore.BP_SaveScore_C"))
  (bind _output_get (Variables|Default|SetSave%20Instance _returnvalue))
  (Variables|/Game/Blueprints/BP_SaveScore.BP_SaveScore_C|SetScoreData _output_get SaveValue)
  ;[1 1 1] 조정한 데이터 저장
  (SaveGame|SaveGametoSlot _output_get "BestScoreData"))

(fn LoadScoreData
  (SaveGame|DoesSaveGameExist)
  (if true
    (bind _returnvalue (SaveGame|LoadGamefromSlot "BestScoreData"))
    (bind _asbp_save_score (Utilities|Casting|CastToBP_SaveScore _returnvalue))
    (return (Variables|/Game/Blueprints/BP_SaveScore.BP_SaveScore_C|GetScoreData _asbp_save_score))))